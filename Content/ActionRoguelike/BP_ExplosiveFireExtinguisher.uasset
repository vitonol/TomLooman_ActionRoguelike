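; Explosive fire extinguisher prop for the ActionRoguelike game that reacts to hits on its mesh.
; Any hit turns on physics simulation for the mesh, and a valid other actor also fires the radial force impulse.
; If that actor has an SAttributeComponent, it loses a small fixed amount of health and the extinguisher starts a short lifespan before removal.
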(event OnComponentHit(Mesh)
  (params (HitComponent :type Primitive%20Component%20Object%20Reference) (OtherActor :type Actor%20Object%20Reference) (OtherComp :type Primitive%20Component%20Object%20Reference) (NormalImpulse :type Vector :default "0, 0, 0") (Hit :type Hit%20Result%20Structure%20%28by%20ref%29))
  (bind _returnvalue (Actor|GetComponentbyClass OtherActor "/Script/ActionRoguelike.SAttributeComponent"))
  (Physics|SetSimulatePhysics (Variables|Character|GetMesh) true)
  (Utilities|IsValid OtherActor
    (:Is%20Valid
      (Class|RadialForceComponent|FireImpulse (Variables|Default|GetRadialForce))
      (Utilities|IsValid _returnvalue
        (:Is%20Valid
          (Class|SAttributeComponent|ApplyHealthChange _returnvalue 0 -5.0)
          (Actor|SetLifeSpan 5.0))))))

(fn ConstructionScript
  (|CallParentFunction))