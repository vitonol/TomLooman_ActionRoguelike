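; BP_BoneFire is an interactable bonfire that acts as a save point.
; Interact sets FireActive, then has the SGameModeBase write the save game, activates the flame particles and prints a confirmation, or an error if the cast fails.
; OnActorLoaded reuses UpdateFlames, which activates the particle system only when FireActive is true.
; GetInteractText returns an empty prompt.
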(event Custom|UpdateFlames
  (if (Variables|Default|GetbFireActive)
    (Components|Activation|Activate (Variables|Default|GetParticleSystem) false)))

(event EventBeginPlay)

(event Collision|EventActorBeginOverlap
  (params (OtherActor :type Actor%20Object%20Reference)))

(event EventTick
  (params (DeltaSeconds :type Float%20%28single-precision%29)))

(event EventInteract
  (params (InstigatorPawn :type Pawn%20Object%20Reference))
  (Variables|Default|SetbFireActive true)
  (bind _assgame_mode_base (Utilities|Casting|CastToSGameModeBase (Game|GetGameMode))
    (:then
      (Class|SGameModeBase|WriteSaveGame _assgame_mode_base)
      (CallFunction|UpdateFlames)
      (Development|PrintString "Saved"))
    (:CastFailed
      (Development|PrintString "Cast To GM FAILED" true true "(R=1.000000,G=0.000000,B=0.000000,A=1.000000)"))))

(event EventOnActorLoaded
  (CallFunction|UpdateFlames))

(fn ConstructionScript)

(fn GetInteractText
  (params (InstigatorPawn :type Pawn%20Object%20Reference))
  (return ""))