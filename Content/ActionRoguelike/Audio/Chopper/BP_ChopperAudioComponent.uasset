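; Audio component for the player-enterable chopper, driving a MotoSynth engine sound and assigning the blades sound.
; Entering the chopper resets RPM and starts the synth.
; Each tick maps blade rotation speed to a target RPM, smooths it, and converts it logarithmically into the synth's RPM range, which also scales volume.
; Forward MPH is stored but unused here; debug RPM prints remain on screen.
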(event Custom|ModulateMotoAccel
  (Audio|Components|Audio|SetVolumeMultiplier (Variables|Default|GetSynthComponentMoto) 0.0 :!class /Script/AudioMixer.SynthComponent))

(event Custom|ModulateMotoDeccel
  (Audio|Components|Audio|SetVolumeMultiplier (Variables|Default|GetSynthComponentMoto) 0.0 :!class /Script/AudioMixer.SynthComponent))

(event Custom|EnterChopper
  (CallFunction|ResetRPMValues)
  (CallFunction|StartMotosynth))

(event EventBeginPlay
  (bind _asbp_chopper (Utilities|Casting|CastToBP_Chopper (Actor|GetParentActor)))
  (Variables|Default|SetCurrentChopper _asbp_chopper)
  (bind _audio (Variables|Default|GetAudio)
    (:then
      (Audio|Components|Audio|SetSound _audio "/Game/ActionRoguelike/Audio/Chopper/MS_Blades.MS_Blades")
      (Variables|/Script/MotoSynth.SynthComponentMoto|SetMotoSynthPreset (Variables|Default|GetSynthComponentMoto) "/Game/ActionRoguelike/Audio/Chopper/MotoSynth/Moto_Preset.Moto_Preset")
      (EventDispatchers|BindEventtoOnPlayerEnterChopper (Variables|Default|GetCurrentChopper) (EventDispatchers|CreateEvent :!event Custom|EnterChopper)))
    (:else)))

(event EventTick
  (params (DeltaSeconds :type Float%20%28single-precision%29))
  (Variables|Default|SetDelta%20Seconds DeltaSeconds)
  (Utilities|FlowControl|Sequence
    (:then_0
      (CallFunction|UpdateEngineRPM)
      (CallFunction|SetCurrentMPH)
      (CallFunction|InterpolateEngineRPM)
      (Class|SynthComponentMoto|SetRPM (Variables|Default|GetSynthComponentMoto) (Variables|Default|GetCurrentMotosynthRPM) (Variables|Default|GetDelta%20Seconds)))
    (:then_1
      (bind (_outminrpm _outmaxrpm) (Class|SynthComponentMoto|GetRPMRange (Variables|Default|GetSynthComponentMoto)))
      (Audio|Components|Audio|SetVolumeMultiplier (Variables|Default|GetSynthComponentMoto) (Math|Float|MapRangeClamped (Math|Float|MapRangeClamped (Variables|Default|GetCurrentMotosynthRPM) _outminrpm _outmaxrpm 0.0 1.0) 0.0 0.1 0.0 1.0) :!class /Script/AudioMixer.SynthComponent))
    (:then_2
      (Development|PrintText (Utilities|Text|FormatText "Target RPM: {Target} 
 
Interp RPM: {Interp} 
 
Current MotoSynth RPM: {moto} 
 
" (Variables|Default|GetTargetRPM) (Variables|Default|GetInterpRPM) (Variables|Default|GetCurrentMotosynthRPM)) true true "(R=1.000000,G=0.523730,B=0.000000,A=1.000000)" 0.0))))

(fn ConstructionScript)

(fn SetCurrentMPH
  (Variables|Default|SetCurrentMPH (Class|SHelicopterSM|GetForwardSpeedMPH (Variables|Default|GetCurrentChopper))))

(fn InterpolateEngineRPM
  (Variables|Default|SetInterpRPM (Math|Interpolation|FInterpTo (Variables|Default|GetInterpRPM) (Variables|Default|GetTargetRPM) (Variables|Default|GetDelta%20Seconds) 3.0))
  (bind (_outminrpm _outmaxrpm) (Class|SynthComponentMoto|GetRPMRange (Variables|Default|GetSynthComponentMoto)))
  (bind _returnvalue (Class|SynthesisUtilitiesBlueprintFunctionLibrary|GetLogFrequency (Variables|Default|GetInterpRPM) 0.0 (- _outmaxrpm 2e+03) _outminrpm _outmaxrpm))
  (Variables|Default|SetCurrentMotosynthRPM _returnvalue)
  (Development|PrintString (Utilities|String|Append (Utilities|String|ToString(Float) _outminrpm) "  / " (Utilities|String|ToString(Float) _outmaxrpm)) true true "(R=1.000000,G=0.000000,B=0.883554,A=1.000000)" 0.0))

(fn StartMotosynth
  (bind _synthcomponentmoto (Variables|Default|GetSynthComponentMoto))
  (Class|SynthComponentMoto|SetRPM _synthcomponentmoto (Variables|Default|GetInterpRPM) (Variables|Default|GetDelta%20Seconds))
  (CameraShake|Start _synthcomponentmoto))

(fn ResetRPMValues
  (Variables|Default|SetInterpRPM 0.0)
  (Variables|Default|SetTargetRPM 0.0))

(fn UpdateEngineRPM
  (Variables|Default|SetTargetRPM (Math|Float|MapRangeClamped (Class|SHelicopterSM|GetBladeRotationSpeed (Variables|Default|GetCurrentChopper)) 0.0 1.5e+03 0.0 (- 1.5e+04 (Variables|Default|GetRPMMaxBuffer%20)))))