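; Pilotable helicopter that a player possesses on Interact, attaching the character to the pilot seat until F ejects and repossesses it.
; Throttle input sets target rotor speed, which eases in and feeds a curve for lift and lift-scaled steering.
; Tick moves it with hand-rolled physics, deriving velocity from position change, adding gravity, tilt-based lift and horizontal thrust, then sweeping.
; Rotors swap to blurred meshes above a speed threshold, capping visible spin.
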(event EventInteract
  (params (InstigatorPawn :type Pawn%20Object%20Reference))
  (bind _asbp_player_character (Utilities|Casting|CastToBP_PlayerCharacter InstigatorPawn))
  (Variables|Private|SetOccupant _asbp_player_character)
  (Pawn|Possess (Pawn|GetController InstigatorPawn) self)
  (Collision|SetCollisionProfileName (Variables|/Script/Engine.Character|GetCapsuleComponent _asbp_player_character) "NoCollision" true :!class /Script/Engine.PrimitiveComponent)
  (Variables|/Game/ActionRoguelike/BP_PlayerCharacter.BP_PlayerCharacter_C|SetbPiloting (Variables|Private|GetOccupant) true)
  (Transformation|AttachActorToActor (Variables|Private|GetOccupant) self "pilot_seat" "SnapToTarget" "SnapToTarget" "SnapToTarget" true))

(event EventTick
  (params (DeltaSeconds :type Float%20%28single-precision%29))
  (Private|TickUpdate DeltaSeconds)
  (Private|RotateBlades DeltaSeconds))

(event EventBeginPlay
  (Private|UpdatePreviousValues))

(event Input|AxisEvents|InputAxisMoveUp
  (params (AxisValue :type Float%20%28single-precision%29))
  (Variables|Private|SetTargetBladeRotationSpeed (Math|Float|Clamp(Float) (+ (* (* AxisValue -1.0) (Utilities|Time|GetWorldDeltaSeconds) (Variables|Constants|GetThrottleUpSpeed)) (Variables|Private|GetTargetBladeRotationSpeed)) 0.0 (Variables|Constants|GetMaxBladeRotationSpeed))))

(event Input|AxisEvents|InputAxisRotateRight
  (params (AxisValue :type Float%20%28single-precision%29))
  (bind _output_get (Variables|Private|SetCurrentRotation (Math|Interpolation|FInterpTo (Variables|Private|GetCurrentRotation) (* AxisValue (Private|GetTurnSpeed)) (Utilities|Time|GetWorldDeltaSeconds) 2.0)))
  (Transformation|AddActorLocalRotation (Math|Rotator|MakeRotator 0.0 0.0 _output_get) false false))

(event Input|AxisEvents|InputAxisTiltForward
  (params (AxisValue :type Float%20%28single-precision%29))
  (bind _output_get (Variables|Private|SetCurrentPitch (Math|Interpolation|FInterpTo (Variables|Private|GetCurrentPitch) (* (* AxisValue -1.0) (Private|GetTurnSpeed)) (Utilities|Time|GetWorldDeltaSeconds) 3.0)))
  (if (Math|Float|InRange(Float) (+ _output_get (.pitch (Transformation|GetActorRotation))) -89.0 89.0)
    (Transformation|AddActorLocalRotation (Math|Rotator|MakeRotator 0.0 _output_get 0.0) false false)))

(event Input|AxisEvents|InputAxisTiltRight
  (params (AxisValue :type Float%20%28single-precision%29))
  (bind _returnvalue (Transformation|GetActorRotation))
  (bind _output_get (Variables|Private|SetCurrentTurn (Math|Interpolation|FInterpTo (Variables|Private|GetCurrentTurn) (* AxisValue (Private|GetTurnSpeed)) (Utilities|Time|GetWorldDeltaSeconds) 2.5)))
  (Class|Actor|AddActorWorldRotation (Math|Rotator|MakeRotator 0.0 0.0 _output_get))
  (Transformation|SetActorRotation (Math|Rotator|MakeRotator (* _output_get 43.0) (.pitch _returnvalue) (.yaw _returnvalue))))

(event Input|KeyboardEvents|F
  (params (Key :type Key%20Structure :default "None"))
  (:Pressed
    (bind _occupant (Variables|Private|GetOccupant)
      (:then
        (Transformation|DetachFromActor _occupant "KeepWorld" "KeepWorld" "KeepWorld")
        (Transformation|SetActorLocation (Variables|Private|GetOccupant) (Transformation|GetWorldLocation (Variables|Default|GetBox1)) false false)
        (Collision|SetCollisionProfileName (Variables|/Script/Engine.Character|GetCapsuleComponent (Variables|Private|GetOccupant)) "Pawn" true :!class /Script/Engine.PrimitiveComponent)
        (Collision|SetCollisionProfileName (Variables|/Script/Engine.Character|GetMesh (Variables|Private|GetOccupant)) "CharacterMesh" true :!class /Script/Engine.PrimitiveComponent)
        (Pawn|Possess (Pawn|GetController) (Variables|Private|GetOccupant))
        (Variables|/Game/ActionRoguelike/BP_PlayerCharacter.BP_PlayerCharacter_C|SetbPiloting (Variables|Private|GetOccupant) false)
        (Variables|Private|SetOccupant 0))
      (:else))))

(fn ConstructionScript)

(fn TickUpdate
  (params (DeltaSeconds :type Float%20%28double-precision%29))
  (bind _returnvalue (Transformation|GetActorUpVector))
  (Utilities|FlowControl|Sequence
    (:then_0
      ;[1 1 1] Update blade rotation Speed to match target
      (Variables|Private|SetCurrentBladeRotationSpeed (Math|Interpolation|FInterpTo (Variables|Private|GetCurrentBladeRotationSpeed) (Variables|Private|GetTargetBladeRotationSpeed) DeltaSeconds 3.0)))
    (:then_1
      ;[1 1 1] Compute Velocity and acceleration
      (Variables|Private|SetVelocity (* (- (Transformation|GetActorLocation) (Variables|Private|GetPrevPosition)) DeltaSeconds))
      (Variables|Private|SetAcceleration (* (- (Variables|Private|GetVelocity) (Variables|Private|GetPrevVelocity)) DeltaSeconds)))
    (:then_2
      (Private|UpdatePreviousValues))
    (:then_3
      ;[1 1 1] Apply Gravity
      (Variables|Private|SetAcceleration (+ (Variables|Private|GetAcceleration) "0.000000,0.000000,-981.000000"))
      ;[1 1 1] Apply Lift
      (Variables|Private|SetAcceleration (+ (Variables|Private|GetAcceleration) (* (Transformation|GetActorUpVector) (Private|GetCurrentLift))))
      ;[1 1 1] Simulate forward acceleration
      (Variables|Private|SetAcceleration (+ (Variables|Private|GetAcceleration) (* (Math|Vector|MakeVector (.x _returnvalue) (.y _returnvalue) 0.0) (* (Private|GetCurrentLift) 2.0)))))
    (:then_4
      ;[1 1 1] Move Helicopter
      (Transformation|AddActorWorldOffset (+ (Variables|Private|GetVelocity) (* (Variables|Private|GetAcceleration) DeltaSeconds)) true))))

(fn RotateBlades
  (params (DeltaSeconds :type Float%20%28double-precision%29))
  (bind _currentbladerotationspeed (Variables|Private|GetCurrentBladeRotationSpeed))
  (bind _blurbladespeedthreshold (Variables|Constants|GetBlurBladeSpeedThreshold))
  (bind _currentbladerotationspeed_2 (Variables|Private|GetCurrentBladeRotationSpeed))
  (bind _blurbladespeedthreshold_2 (Variables|Constants|GetBlurBladeSpeedThreshold))
  (bind _returnvalue (> _currentbladerotationspeed_2 _blurbladespeedthreshold_2))
  (bind _returnvalue_2 (Math|Float|SelectFloat _blurbladespeedthreshold _currentbladerotationspeed _returnvalue))
  (bind _returnvalue_3 (* _returnvalue_2 DeltaSeconds))
  (if _returnvalue
    (Components|StaticMesh|SetStaticMesh (Variables|Default|GetBlade) "/Game/ActionRoguelike/Heli/Assets/main_rotor_blade_blur.main_rotor_blade_blur")
    (Components|StaticMesh|SetStaticMesh (Variables|Default|GetTailBlade) "/Game/ActionRoguelike/Heli/Assets/tail_rotor_blade_blur.tail_rotor_blade_blur")
    (else
      (Components|StaticMesh|SetStaticMesh (Variables|Default|GetBlade) "/Game/ActionRoguelike/Heli/Assets/main_rotor_blade.main_rotor_blade")
      (Components|StaticMesh|SetStaticMesh (Variables|Default|GetTailBlade) "/Game/ActionRoguelike/Heli/Assets/rear_rotor_blade.rear_rotor_blade")))
  (Transformation|AddRelativeRotation (Variables|Default|GetRotor) (Math|Rotator|MakeRotator 0.0 0.0 _returnvalue_3) false false)
  (Transformation|AddLocalRotation (Variables|Default|GetTailRotor) (Math|Rotator|MakeRotator 0.0 (* _returnvalue_3 2.0) 0.0) false false))

(fn GetCurrentLift
  (return (Math|Curves|GetFloatValue (Variables|Constants|GetLiftCurve) (Variables|Private|GetCurrentBladeRotationSpeed))))

(fn UpdatePreviousValues
  (Variables|Private|SetPrevPosition (Transformation|GetActorLocation))
  (Variables|Private|SetPrevVelocity (Variables|Private|GetVelocity))
  (Variables|Private|SetPrevAcceleration (Variables|Private|GetAcceleration)))

(fn GetTurnSpeed
  (return (* (Variables|Constants|GetTurnSpeed) (Math|Float|MapRangeClamped (Private|GetCurrentLift) 0.0 4e+02 0.0 1.0))))