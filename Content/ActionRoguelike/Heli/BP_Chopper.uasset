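; Helicopter pawn Blueprint that adds player-possession setup and rotor visuals to its parent class.
; When a BP_PlayerController possesses it, it sets the chopper audio component class on a child actor component and removes the player character's health widget from its parent.
; The construction script snaps both rotors to body mesh sockets.
; Cosmetic events swap main and tail blade meshes between normal and blurred versions.
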(event EventBeginPlay
  (|CallParentFunction))

(event EventTick
  (params (DeltaSeconds :type Float%20%28single-precision%29)))

(event EventPossessed
  (params (NewController :type Controller%20Object%20Reference))
  (Utilities|Casting|CastToBP_PlayerController NewController)
  (ChildActorComponent|SetChildActorClass (Variables|Default|GetBP_AudioController) "/Game/ActionRoguelike/Audio/Chopper/BP_ChopperAudioComponent.BP_ChopperAudioComponent_C")
  (bind _returnvalue (Actor|GetActorOfClass "/Game/ActionRoguelike/BP_PlayerCharacter.BP_PlayerCharacter_C"))
  (Widget|RemovefromParent (Variables|/Game/ActionRoguelike/BP_PlayerCharacter.BP_PlayerCharacter_C|GetHealthWidget _returnvalue)))

(event EventLoadBlurryBladeMesh
  (Components|StaticMesh|SetStaticMesh (Variables|Default|GetMeshBlade) "/Game/ActionRoguelike/Heli/Assets/main_rotor_blade_blur.main_rotor_blade_blur")
  (Components|StaticMesh|SetStaticMesh (Variables|Default|GetMeshTailBlade) "/Game/ActionRoguelike/Heli/Assets/tail_rotor_blade_blur.tail_rotor_blade_blur"))

(event EventLoadNormalBladeMesh
  (Components|StaticMesh|SetStaticMesh (Variables|Default|GetMeshBlade) "/Game/ActionRoguelike/Heli/Assets/main_rotor_blade.main_rotor_blade")
  (Components|StaticMesh|SetStaticMesh (Variables|Default|GetMeshTailBlade) "/Game/ActionRoguelike/Heli/Assets/rear_rotor_blade.rear_rotor_blade"))

(fn ConstructionScript
  (bind _output_get (Variables|Default|SetTailRotorSocket "tail_rotor"))
  (bind _output_get_2 (Variables|Default|SetRotorSocket "main_rotor"))
  (Transformation|AttachComponentToComponent (Variables|Default|GetMeshTailRotor) (Variables|Default|GetMeshBody) "tail_rotor" "SnapToTarget" "SnapToTarget" "SnapToTarget" false)
  (Transformation|AttachComponentToComponent (Variables|Default|GetMeshRotor) (Variables|Default|GetMeshBody) "main_rotor" "SnapToTarget" "SnapToTarget" "SnapToTarget" false))